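; BP_Ball is a character ball that is placed at a fixed start location on BeginPlay.
; BeginPlay also shows the mouse cursor, then lowers CharacterMovement gravity after a delay so the ball is only lightly pulled.
; Touch-drag logic for tracking finger deltas and moving the ball within clamped bounds is present but disconnected, and the TouchDrag event is empty.
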(event Custom|TouchDrag)

(event EventBeginPlay
  (Variables|/Script/Engine.PlayerController|SetbShowMouseCursor (Game|GetPlayerController 0) true)
  (Transformation|SetActorLocation "-72.500000, 0, 0" false false)
  (Utilities|FlowControl|Delay 5.0)
  (Variables|/Script/Engine.CharacterMovementComponent|SetGravityScale (Variables|Character|GetCharacterMovement) 0.1))

(event Input|TouchEvents|InputTouch
  (params (Location :type Vector) (FingerIndex :type ETouchIndex%20Enum)))

(fn ConstructionScript)