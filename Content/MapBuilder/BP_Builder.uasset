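; BP_Builder builds the selected level for the ball game as a vertical column of walls ending in a floor.
; On BeginPlay it reads the selected level's info to set the player ball's gravity scale as difficulty and the depth to build to.
; Spawn then stacks numbered wall segments downward at fixed intervals to that depth and caps them with a floor, passing each piece the level's materials.
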(event Custom|Spawn
  (bind _s_levelinfo (Variables|Default|GetS_LevelInfo))
  (bind _levelselected (Variables|Default|GetLevelSelected))
  (bind _output (Utilities|Array|Get(acopy) _s_levelinfo _levelselected))
  (bind (_distancetospawn _wallmaterial _backgroundmaterial _floormaterial _difficultyscale) (Utilities|Struct|BreakS_LevelInfo _output))
  (Game|SpawnActorfromClass "/Game/MapBuilder/Templates/BP_Wall_Base.BP_Wall_Base_C" (Math|Transform|MakeTransform "0, 0, 0" "0, 0, 0" "1,1,1") "Undefined" 0 (Variables|Default|GetCount) _wallmaterial _backgroundmaterial 0)
  (Math|Integer|IncrementInt (Variables|Default|GetCount)
    (:%20%20
      (while (> (Variables|Default|GetLastHeight) (Variables|Default|GetDistanceToSpawn))
        (Game|SpawnActorfromClass "/Game/MapBuilder/Templates/BP_Wall_Base.BP_Wall_Base_C" (Math|Transform|MakeTransform (Math|Vector|MakeVector 0.0 0.0 (- (Variables|Default|GetLastHeight) 5e+02)) "0, 0, 0" "1,1,1") "Undefined" 0 (Variables|Default|GetCount) _wallmaterial _backgroundmaterial 0)
        (Variables|Default|SetLastHeight (- (Variables|Default|GetLastHeight) 5e+02))
        (Math|Integer|IncrementInt (Variables|Default|GetCount)))
      (Game|SpawnActorfromClass "/Game/MapBuilder/Templates/BP_Floor_Base.BP_Floor_Base_C" (Math|Transform|MakeTransform (Math|Vector|MakeVector 0.0 0.0 (- (Variables|Default|GetLastHeight) 5e+02)) "0, 0, 0" "1,1,1") "Undefined" 0 0 _wallmaterial _backgroundmaterial _floormaterial 0))))

(event EventBeginPlay
  (bind _s_levelinfo (Variables|Default|GetS_LevelInfo))
  (bind _levelselected (Variables|Default|GetLevelSelected))
  (bind _output (Utilities|Array|Get(acopy) _s_levelinfo _levelselected))
  (bind (_distancetospawn _wallmaterial _backgroundmaterial _floormaterial _difficultyscale) (Utilities|Struct|BreakS_LevelInfo _output))
  (bind _asbp_ball (Utilities|Casting|CastToBP_Ball (Game|GetPlayerCharacter 0)))
  (Variables|/Game/Character/BP_Ball.BP_Ball_C|SetGravityScale _asbp_ball _difficultyscale)
  (Variables|Default|SetDistanceToSpawn _distancetospawn)
  (CallFunction|Spawn))

(fn ConstructionScript)