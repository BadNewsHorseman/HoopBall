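; Demo controller for cartoony UI animations, opening on the main menu and switching between main menu, in-game, shop, level cleared and level select screens via number keys.
; Each screen event clears all widgets, creates and displays its widget, then plays that screen's animations.
; Looping MultiGates cycle animation variants on each replay, with delays sequencing follow-ups and a random gate picking one to three level-cleared stars.
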(event Custom|Main%20menu
  (Viewport|RemoveAllWidgets)
  ;[1 1 1] Create Main Menu and save reference of it, and add it to the screen
  (bind _returnvalue (UserInterface|CreateWidget "/Game/Cartoony_UI_Anims/UI/UI_MainMenu.UI_MainMenu_C"))
  (bind _output_get (Variables|Default|SetMain%20Menu%20UI _returnvalue))
  (UserInterface|Viewport|AddtoViewport _output_get 0)
  ;[1 1 1] Start playing animations
  (CallFunction|PlayMainMenuAnims))

(event Custom|In-Game
  (Viewport|RemoveAllWidgets)
  ;[1 1 1] Create Main Menu and save reference of it, and add it to the screen
  (bind _returnvalue (UserInterface|CreateWidget "/Game/Cartoony_UI_Anims/UI/UI_In-Game.UI_In-Game_C"))
  (bind _output_get (Variables|Default|SetIn-Game%20UI _returnvalue))
  (UserInterface|Viewport|AddtoViewport _output_get 0)
  ;[1 1 1] Start playing animations
  (CallFunction|PlayIn-GameAnim))

(event Custom|Shop
  (Viewport|RemoveAllWidgets)
  ;[1 1 1] Create Main Menu and save reference of it, and add it to the screen
  (bind _returnvalue (UserInterface|CreateWidget "/Game/Cartoony_UI_Anims/UI/UI_Shop.UI_Shop_C"))
  (bind _output_get (Variables|Default|SetShop%20UI _returnvalue))
  (UserInterface|Viewport|AddtoViewport _output_get 0)
  ;[1 1 1] Start playing animations
  (CallFunction|PlayShopAnim))

(event Custom|Level%20Cleared
  (Viewport|RemoveAllWidgets)
  ;[1 1 1] Create Main Menu and save reference of it, and add it to the screen
  (bind _returnvalue (UserInterface|CreateWidget "/Game/Cartoony_UI_Anims/UI/UI_LevelCleared.UI_LevelCleared_C"))
  (bind _output_get (Variables|Default|SetLevelCleared%20UI _returnvalue))
  (UserInterface|Viewport|AddtoViewport _output_get 0)
  ;[1 1 1] Start playing animations
  (CallFunction|PlayLevelClearedAnims))

(event Custom|Level%20Select
  (Viewport|RemoveAllWidgets)
  ;[1 1 1] Create Main Menu and save reference of it, and add it to the screen
  (bind _returnvalue (UserInterface|CreateWidget "/Game/Cartoony_UI_Anims/UI/UI_LevelSelect.UI_LevelSelect_C"))
  (bind _output_get (Variables|Default|SetLevel%20Select%20UI _returnvalue))
  (UserInterface|Viewport|AddtoViewport _output_get 0)
  ;[1 1 1] Start playing animations
  (CallFunction|LevelSelectAnims))

(event EventBeginPlay
  (|Mouseinteratcionsetup
    (:%20
      (CallFunction|MainMenu))))

(event EventTick
  (params (DeltaSeconds :type Float%20%28single-precision%29)))

(event Input|KeyboardEvents|1
  (params (Key :type Key%20Structure))
  (:Pressed
    (CallFunction|MainMenu)))

(event Input|KeyboardEvents|4
  (params (Key :type Key%20Structure))
  (:Pressed
    (CallFunction|LevelCleared)))

(event Input|KeyboardEvents|5
  (params (Key :type Key%20Structure))
  (:Pressed
    (CallFunction|LevelSelect)))

(event Input|KeyboardEvents|SpaceBar
  (params (Key :type Key%20Structure))
  (:Pressed
    (CallFunction|LevelCleared)))

(event Input|KeyboardEvents|2
  (params (Key :type Key%20Structure))
  (:Pressed
    (CallFunction|In-Game)))

(event Input|KeyboardEvents|3
  (params (Key :type Key%20Structure))
  (:Pressed
    (CallFunction|Shop)))

(fn ConstructionScript)

(event Custom|Play%20Main%20Menu%20Anims
  (bind _main_menu_ui (Variables|Default|GetMain%20Menu%20UI))
  (bind _main_menu_ui_2 (Variables|Default|GetMain%20Menu%20UI))
  (bind _main_menu_ui_3 (Variables|Default|GetMain%20Menu%20UI))
  (bind _main_menu_ui_4 (Variables|Default|GetMain%20Menu%20UI))
  (bind _main_menu_ui_5 (Variables|Default|GetMain%20Menu%20UI))
  ;[1 1 1] Play Animation of the play button
  (Utilities|FlowControl|MultiGate false true -1
    (:Out%200
      (UserInterface|Animation|PlayAnimation _main_menu_ui_3 (Variables|/Game/Cartoony_UI_Anims/UI/UI_MainMenu.UI_MainMenu_C|GetPlayButton%20Bubble _main_menu_ui_3) 0.0 1 "Forward" 1.0)
      (Utilities|FlowControl|Delay 0.65))
    (:Out%201
      (UserInterface|Animation|PlayAnimation _main_menu_ui_3 (Variables|/Game/Cartoony_UI_Anims/UI/UI_MainMenu.UI_MainMenu_C|GetPlayButton%20Jump _main_menu_ui_3) 0.0 1 "Forward" 1.0)
      ;[1 1 1] wait for anim to finish
      (Utilities|FlowControl|Delay 0.75))
    (:Out%202
      (UserInterface|Animation|PlayAnimation _main_menu_ui_3 (Variables|/Game/Cartoony_UI_Anims/UI/UI_MainMenu.UI_MainMenu_C|GetPlayButtonSkewFall _main_menu_ui_3) 0.0 1 "Forward" 1.0)
      (Utilities|FlowControl|Delay 0.8)))
  (Utilities|FlowControl|Sequence
    (:then_0
      ;[1 1 1] Make Play button pulse infinitely
      (UserInterface|Animation|PlayAnimation _main_menu_ui (Variables|/Game/Cartoony_UI_Anims/UI/UI_MainMenu.UI_MainMenu_C|GetPlayButton%20Heartbeat _main_menu_ui) 0.0 0 "Forward" 1.0))
    (:then_1
      (Utilities|FlowControl|MultiGate false true -1
        (:Out%200
          (UserInterface|Animation|PlayAnimation _main_menu_ui_5 (Variables|/Game/Cartoony_UI_Anims/UI/UI_MainMenu.UI_MainMenu_C|GetBottomButtons%20Contant%20Grow _main_menu_ui_5) 0.0 1 "Forward" 1.4))
        (:Out%201
          (UserInterface|Animation|PlayAnimation _main_menu_ui_5 (Variables|/Game/Cartoony_UI_Anims/UI/UI_MainMenu.UI_MainMenu_C|GetBottomButtons%20Instant%20Grow _main_menu_ui_5) 0.0 1 "Forward" 1.2))
        (:Out%202
          (UserInterface|Animation|PlayAnimation _main_menu_ui_5 (Variables|/Game/Cartoony_UI_Anims/UI/UI_MainMenu.UI_MainMenu_C|GetBottomButtons%20Skew _main_menu_ui_5) 0.0 1 "Forward" 1.7))))
    (:then_2
      (UserInterface|Animation|PlayAnimation _main_menu_ui_2 (Variables|/Game/Cartoony_UI_Anims/UI/UI_MainMenu.UI_MainMenu_C|GetGameTitleSkewBounce _main_menu_ui_2) 0.0 1 "Forward" 1.0)
      (Widget|SetVisibility (Variables|/Game/Cartoony_UI_Anims/UI/UI_MainMenu.UI_MainMenu_C|GetDemoGame _main_menu_ui_2) "HitTestInvisible")
      (UserInterface|Animation|PlayAnimation _main_menu_ui_2 (Variables|/Game/Cartoony_UI_Anims/UI/UI_MainMenu.UI_MainMenu_C|GetSunrayZoomIn _main_menu_ui_2) 0.0 1 "Forward" 1.0)
      (Widget|SetVisibility (Variables|/Game/Cartoony_UI_Anims/UI/UI_MainMenu.UI_MainMenu_C|GetSunray1 _main_menu_ui_2) "HitTestInvisible")
      (Widget|SetVisibility (Variables|/Game/Cartoony_UI_Anims/UI/UI_MainMenu.UI_MainMenu_C|GetSunray2 _main_menu_ui_2) "HitTestInvisible")
      ;[1 1 1] Make sunray in the background loop endlessly
      (UserInterface|Animation|PlayAnimation _main_menu_ui_4 (Variables|/Game/Cartoony_UI_Anims/UI/UI_MainMenu.UI_MainMenu_C|GetSunRayRotate _main_menu_ui_4) 0.0 0 "Forward" 1.0))))

(event Custom|Play%20Shop%20Anim
  (bind _shop_ui (Variables|Default|GetShop%20UI))
  ;[1 1 1] Shop Anim
  (Utilities|FlowControl|MultiGate false true -1
    (:Out%200
      (UserInterface|Animation|PlayAnimation _shop_ui (Variables|/Game/Cartoony_UI_Anims/UI/UI_Shop.UI_Shop_C|GetOpenShop%20Panel%20Bounce _shop_ui) 0.0 1 "Forward" 1.0))
    (:Out%201
      (UserInterface|Animation|PlayAnimation _shop_ui (Variables|/Game/Cartoony_UI_Anims/UI/UI_Shop.UI_Shop_C|GetOpenShop%20Panel%20Drop%20Bounce _shop_ui) 0.0 1 "Forward" 1.0))
    (:Out%202
      (UserInterface|Animation|PlayAnimation _shop_ui (Variables|/Game/Cartoony_UI_Anims/UI/UI_Shop.UI_Shop_C|GetOpenShop%20Panel%20Drop%20Simple _shop_ui) 0.0 1 "Forward" 1.0))
    (:Out%203
      (UserInterface|Animation|PlayAnimation _shop_ui (Variables|/Game/Cartoony_UI_Anims/UI/UI_Shop.UI_Shop_C|GetOpenShop%20Panel%20Skew _shop_ui) 0.0 1 "Forward" 1.0))))

(event Custom|Play%20In-Game%20Anim
  (bind _in_game_ui (Variables|Default|GetIn-Game%20UI))
  (UserInterface|Animation|PlayAnimation _in_game_ui (Variables|/Game/Cartoony_UI_Anims/UI/UI_In-Game.UI_In-Game_C|GetSlide%20In _in_game_ui) 0.0 1 "Forward" 1.0))

(event Custom|Play%20Level%20Cleared%20Anims
  (bind _levelcleared_ui (Variables|Default|GetLevelCleared%20UI))
  (bind _levelcleared_ui_2 (Variables|Default|GetLevelCleared%20UI))
  (bind _star1anim (Variables|/Game/Cartoony_UI_Anims/UI/UI_LevelCleared.UI_LevelCleared_C|GetStar1Anim _levelcleared_ui_2))
  (bind _star2anim (Variables|/Game/Cartoony_UI_Anims/UI/UI_LevelCleared.UI_LevelCleared_C|GetStar2Anim _levelcleared_ui_2))
  (Utilities|FlowControl|MultiGate false true -1
    (:Out%200
      (UserInterface|Animation|PlayAnimation _levelcleared_ui (Variables|/Game/Cartoony_UI_Anims/UI/UI_LevelCleared.UI_LevelCleared_C|GetOpenPanelAnimSkew _levelcleared_ui) 0.0 1 "Forward" 1.0)
      (Utilities|FlowControl|Delay 0.55))
    (:Out%201
      (UserInterface|Animation|PlayAnimation _levelcleared_ui (Variables|/Game/Cartoony_UI_Anims/UI/UI_LevelCleared.UI_LevelCleared_C|GetOpenPanelAnimScale _levelcleared_ui) 0.0 1 "Forward" 1.0)
      (Utilities|FlowControl|Delay 0.45))
    (:Out%202
      (UserInterface|Animation|PlayAnimation _levelcleared_ui (Variables|/Game/Cartoony_UI_Anims/UI/UI_LevelCleared.UI_LevelCleared_C|GetOpenPanelAnimBounce _levelcleared_ui) 0.0 1 "Forward" 1.0)
      (Utilities|FlowControl|Delay 0.9)))
  (Utilities|FlowControl|MultiGate true true -1
    (:Out%200
      (UserInterface|Animation|PlayAnimation _levelcleared_ui_2 _star1anim 0.0 1 "Forward" 1.0))
    (:Out%201
      (UserInterface|Animation|PlayAnimation _levelcleared_ui_2 _star1anim 0.0 1 "Forward" 1.0)
      (Utilities|FlowControl|Delay 0.2)
      (UserInterface|Animation|PlayAnimation _levelcleared_ui_2 _star2anim 0.0 1 "Forward" 1.0))
    (:Out%202
      (UserInterface|Animation|PlayAnimation _levelcleared_ui_2 _star1anim 0.0 1 "Forward" 1.0)
      (Utilities|FlowControl|Delay 0.2)
      (UserInterface|Animation|PlayAnimation _levelcleared_ui_2 _star2anim 0.0 1 "Forward" 1.0)
      (Utilities|FlowControl|Delay 0.2)
      (UserInterface|Animation|PlayAnimation _levelcleared_ui_2 (Variables|/Game/Cartoony_UI_Anims/UI/UI_LevelCleared.UI_LevelCleared_C|GetStar3Anim _levelcleared_ui_2) 0.0 1 "Forward" 1.0))))

(event Custom|Level%20Select%20Anims
  (bind _level_select_ui (Variables|Default|GetLevel%20Select%20UI))
  ;[1 1 1] Level Select Anims
  (UserInterface|Animation|PlayAnimation _level_select_ui (Variables|/Game/Cartoony_UI_Anims/UI/UI_LevelSelect.UI_LevelSelect_C|GetOpenPanel%20Anim%20Bounce%20Scale _level_select_ui) 0.0 1 "Forward" 1.0))